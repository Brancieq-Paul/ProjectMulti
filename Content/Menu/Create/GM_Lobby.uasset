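; Lobby game mode that gathers players and launches the selected game for the party.
; Login and logout events maintain the controller list, with login also printing session and player counts for debugging.
; SetLvl stores the chosen game, and StartParty requires that selection plus at least two players, printing a message otherwise.
; On start, it removes all widgets and runs a serverTravel console command to the chosen game.
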(event Custom|RmvHUD
  (Viewport|RemoveAllWidgets))

(event Custom|SetLvl
  (params (SelecGame :type Text))
  (Variables|Default|SetSelecGame SelecGame)
  (Variables|Default|SetGameSet true))

(event Custom|StartParty
  (if (>= (Utilities|Array|Length (Variables|Default|GetControllers)) 2)
    (if (Variables|Default|GetGameSet)
      (CallFunction|RmvHUD)
      (Development|ExecuteConsoleCommand (Utilities|String|Append "serverTravel " (Utilities|String|ToString(Text) (Variables|Default|GetSelecGame))) 0)
      (else
        (Development|PrintString "No Game Selected")))
    (else
      (Development|PrintString "You must be at least 2 players"))))

(event EventBeginPlay)

(event EventTick
  (params (DeltaSeconds :type Float%20%28single-precision%29)))

(event EventPostLogin
  (params (NewPlayer :type Player%20Controller%20Object%20Reference))
  (Utilities|Array|AddUnique (Variables|Default|GetControllers) NewPlayer)
  (bind _numconnections (Class|AdvancedSessionsLibrary|GetSessionSettings)
    (:OnSuccess
      (Development|PrintString (Utilities|String|ToString(Integer) _numconnections))
      (Development|PrintText (Utilities|Text|ToText(Integer) (Utilities|Array|Length (Variables|Default|GetControllers)))))))

(event EventOnLogout
  (params (ExitingController :type Controller%20Object%20Reference))
  (bind _asplayer_controller (Utilities|Casting|CastToPlayerController ExitingController))
  (Utilities|Array|RemoveItem (Variables|Default|GetControllers) _asplayer_controller))

(fn ConstructionScript)